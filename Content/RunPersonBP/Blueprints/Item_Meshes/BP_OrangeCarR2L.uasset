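; BP_OrangeCarR2L is a looping traffic car that drives along negative world Y, right to left going by its name.
; BeginPlay caches the OrangeCar component's start location and starts a 0.001-second looping timer that shifts it by CarSpeed per tick, not scaled by delta time.
; GetResetCheck flags when truncated absolute Y exceeds the start's, so the car teleports back, assuming a route mirrored around world Y zero.
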(event Custom|Move
  (bind _orangecar (Variables|Default|GetOrangeCar))
  (bind _returnvalue (Transformation|GetWorldLocation _orangecar))
  (Transformation|SetWorldLocation _orangecar (Math|Vector|MakeVector (.x _returnvalue) (- (.y _returnvalue) (Variables|Default|GetCarSpeed)) (.z _returnvalue)) false false)
  (CallFunction|GetResetCheck)
  (if (Variables|Default|GetResetCheck)
    (Transformation|SetWorldLocation (Variables|Default|GetOrangeCar) (Variables|Default|GetVehicleStartLocation) false true)))

(event EventBeginPlay
  (Utilities|Time|SetTimerbyEvent (delegate Custom|Move) 0.001 true)
  (if (not (Variables|Default|GetLocationCheck))
    (Variables|Default|SetVehicleStartLocation (Transformation|GetWorldLocation (Variables|Default|GetOrangeCar)))
    (Variables|Default|SetLocationCheck true)))

(fn ConstructionScript)

(fn GetResetCheck
  (Variables|Default|SetResetCheck (< (- (Math|Integer|Absolute(Integer) (Math|Float|Truncate (.y (Variables|Default|GetVehicleStartLocation)))) (Math|Integer|Absolute(Integer) (Math|Float|Truncate (.y (Transformation|GetWorldLocation (Variables|Default|GetOrangeCar)))))) 0)))