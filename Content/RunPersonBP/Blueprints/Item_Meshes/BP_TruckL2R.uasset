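; BP_TruckL2R is a looping truck hazard that drives along world Y and kills any RunCharacter it hits.
; A fast looping timer shifts the Truck by CarSpeed until its absolute Y exceeds the start's, assuming a lane centered on world Y zero.
; It then teleports back, usually replaying the engine sound.
; Hits randomly trigger either the run-into or squish death.
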(event OnComponentHit(Truck)
  (params (HitComponent :type Primitive%20Component%20Object%20Reference) (OtherActor :type Actor%20Object%20Reference) (OtherComp :type Primitive%20Component%20Object%20Reference) (NormalImpulse :type Vector :default "0, 0, 0") (Hit :type Hit%20Result%20Structure%20%28by%20ref%29))
  (bind _asrun_character (Utilities|Casting|CastToRunCharacter OtherActor))
  (if (Math|Random|RandomBool)
    (Default|DeathbyRunIntoVehicle _asrun_character)
    (else
      (Default|DeathbyVechileSquish _asrun_character))))

(event Custom|Move
  (bind _truck (Variables|Default|GetTruck))
  (bind _returnvalue (Transformation|GetWorldLocation _truck))
  (Transformation|SetWorldLocation _truck (Math|Vector|MakeVector (.x _returnvalue) (+ (.y _returnvalue) (Variables|Default|GetCarSpeed)) (.z _returnvalue)) false false)
  (CallFunction|GetResetCheck)
  (if (Variables|Default|GetResetCheck)
    (Transformation|SetWorldLocation (Variables|Default|GetTruck) (Variables|Default|GetVehicleStartLocation) false true)
    (if (Math|Random|RandomBoolwithWeight 0.8)
      (Audio|PlaySoundatLocation "/Game/RunPersonBP/Sounds/car-engine-loop-deep.car-engine-loop-deep" (Transformation|GetActorLocation) "0, 0, 0" 0.5 1.0 0.0 0 0 0))))

(event EventBeginPlay
  (Utilities|Time|SetTimerbyEvent (delegate Custom|Move) 0.001 true)
  (if (not (Variables|Default|GetLocationCheck))
    (Variables|Default|SetVehicleStartLocation (Transformation|GetWorldLocation (Variables|Default|GetTruck)))
    (Variables|Default|SetLocationCheck true)
    (Audio|PlaySoundatLocation "/Game/RunPersonBP/Sounds/car-engine-loop-deep.car-engine-loop-deep" (Transformation|GetActorLocation) "0, 0, 0" 0.5 1.0 0.0 0 0 0)))

(fn ConstructionScript)

(fn GetResetCheck
  (Variables|Default|SetResetCheck (< (- (Math|Integer|Absolute(Integer) (Math|Float|Truncate (.y (Variables|Default|GetVehicleStartLocation)))) (Math|Integer|Absolute(Integer) (Math|Float|Truncate (.y (Transformation|GetWorldLocation (Variables|Default|GetTruck)))))) 0)))