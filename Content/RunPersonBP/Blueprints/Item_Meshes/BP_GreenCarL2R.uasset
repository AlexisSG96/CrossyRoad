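; BP_GreenCarL2R is a green car hazard that drives repeatedly along the Y axis and kills the RunCharacter on hit.
; A fast looping timer moves the car mesh by CarSpeed each tick, starting from a location cached at BeginPlay.
; GetResetCheck teleports it back once its absolute Y exceeds the start's, so the lane mirrors around world Y zero, with an occasional horn on reset.
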(event OnComponentHit(GreenCar)
  (params (HitComponent :type Primitive%20Component%20Object%20Reference) (OtherActor :type Actor%20Object%20Reference) (OtherComp :type Primitive%20Component%20Object%20Reference) (NormalImpulse :type Vector :default "0, 0, 0") (Hit :type Hit%20Result%20Structure%20%28by%20ref%29))
  (bind _asrun_character (Utilities|Casting|CastToRunCharacter OtherActor))
  (Default|DeathbyHitVehicle _asrun_character))

(event Custom|Move
  (bind _greencar (Variables|Default|GetGreenCar))
  (bind _returnvalue (Transformation|GetWorldLocation _greencar))
  (Transformation|SetWorldLocation _greencar (Math|Vector|MakeVector (.x _returnvalue) (+ (.y _returnvalue) (Variables|Default|GetCarSpeed)) (.z _returnvalue)) false false)
  (CallFunction|GetResetCheck)
  (if (Variables|Default|GetResetCheck)
    (Transformation|SetWorldLocation (Variables|Default|GetGreenCar) (Variables|Default|GetVehicleStartLocation) false true)
    (if (Math|Random|RandomBoolwithWeight 0.1)
      (Audio|PlaySoundatLocation "/Game/RunPersonBP/Sounds/car-horn.car-horn" (Transformation|GetActorLocation) "0, 0, 0" 0.5 1.0 0.0 0 0 0))))

(event EventBeginPlay
  (Utilities|Time|SetTimerbyEvent (delegate Custom|Move) 0.001 true)
  (if (not (Variables|Default|GetLocationCheck))
    (Variables|Default|SetVehicleStartLocation (Transformation|GetWorldLocation (Variables|Default|GetGreenCar)))
    (Variables|Default|SetLocationCheck true)))

(fn ConstructionScript)

(fn GetResetCheck
  (Variables|Default|SetResetCheck (< (- (Math|Integer|Absolute(Integer) (Math|Float|Truncate (.y (Variables|Default|GetVehicleStartLocation)))) (Math|Integer|Absolute(Integer) (Math|Float|Truncate (.y (Transformation|GetWorldLocation (Variables|Default|GetGreenCar)))))) 0)))