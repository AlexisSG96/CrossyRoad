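; Game mode for a lane-based level of grass and road tiles that shows the title widget and builds the course on BeginPlay.
; It spawns a start area, then chains a fixed run of random tiles picked from DifferentFloorTiles.
; Each spawned piece is cast to its class (start area, grass, or either road direction) so its attach transform becomes the next spawn point.
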(event EventBeginPlay
  (bind _returnvalue (UserInterface|CreateWidget "/Game/RunPersonBP/UMG/TitleWidget.TitleWidget_C"))
  (UserInterface|Viewport|AddtoViewport _returnvalue 0)
  (CallFunction|AddStartArea)
  (for _index (range 0 80)
    (CallFunction|AddFloorTile)))

(fn ConstructionScript)

(fn AddFloorTile
  (bind _differentfloortiles (Variables|Default|GetDifferentFloorTiles))
  (bind _returnvalue (Game|SpawnActorfromClass (Utilities|Array|Get(acopy) _differentfloortiles (Math|Random|RandomIntegerinRange 0 (Utilities|Array|LastIndex _differentfloortiles))) (Variables|Default|GetNextSpawnPoint) "Undefined" 0 0))
  (bind _output_get (Variables|Default|SetBlueprintRef _returnvalue))
  (bind _asbp_grass (Utilities|Casting|CastToBP_Grass _output_get)
    (:then
      (bind _attachtransform (Default|GetAttachTransform _asbp_grass))
      (Variables|Default|SetNextSpawnPoint _attachtransform))
    (:CastFailed
      (bind _asbp_road_left_to_right (Utilities|Casting|CastToBP_RoadLeftToRight (Variables|Default|GetBlueprintRef))
        (:then
          (bind _attachtransform_2 (Default|GetAttachTransform _asbp_road_left_to_right))
          (Variables|Default|SetNextSpawnPoint _attachtransform_2))
        (:CastFailed
          (bind _asbp_road_right_to_left (Utilities|Casting|CastToBP_RoadRightToLeft (Variables|Default|GetBlueprintRef)))
          (bind _attachtransform_3 (Default|GetAttachTransform _asbp_road_right_to_left))
          (Variables|Default|SetNextSpawnPoint _attachtransform_3))))))

(fn AddStartArea
  (bind _returnvalue (Game|SpawnActorfromClass "/Game/RunPersonBP/Blueprints/BP_StartArea.BP_StartArea_C" (Variables|Default|GetNextSpawnPoint) "Undefined" 0 0))
  (bind _asbp_start_area (Utilities|Casting|CastToBP_StartArea _returnvalue))
  (bind _attachtransform (Default|GetAttachTransform _asbp_start_area))
  (Variables|Default|SetNextSpawnPoint _attachtransform))